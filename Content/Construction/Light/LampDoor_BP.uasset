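; Door indicator lamp whose point light color shows whether its linked door is blocked.
; On BeginPlay it finds the linked door's DoorComponent_Basic, binds to its block and unblock events, and sets its initial state from IsBlocked.
; Lock and Unlock update the Locked flag and switch the light between the locked and unlocked colors, so the lamp follows door events without ticking.
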(event `self.ReceiveBeginPlay`
  (bind _doorlinked (`self.DoorLinked`))
  (bind _returnvalue (`self.GetComponentByClass` _doorlinked "/Script/Erebe.DoorComponent_Basic"))
  (`/Engine/EditorBlueprintResources/StandardMacros.IsValid` _doorlinked
    (:`Is Valid`
      (`/Engine/EditorBlueprintResources/StandardMacros.IsValid` _returnvalue
        (:`Is Valid`
          (add `DoorComponent_Basic.OnDoorBlock` _returnvalue (delegate `OnLinkedDoorBlock`))
          (add `DoorComponent_Basic.OnDoorUnblock` _returnvalue (delegate `OnLinkedDorrUnblock`))
          (if (`DoorComponent_Basic.bIsBlocked` _returnvalue)
            (`self.Lock`)
            (else
              (`self.Unlock`))))))))

(event `OnLinkedDoorBlock`
  (`self.Lock`))

(event `OnLinkedDorrUnblock`
  (`self.Unlock`))

(fn `ChangeColorFromLocked`
  (bind _pointlight (`self.PointLight`))
  (if (`self.Locked`)
    (`LightComponent.SetLightColor` _pointlight (`self.LockedColor`) true)
    (else
      (`LightComponent.SetLightColor` _pointlight (`self.UnlockedColor`) true))))

(fn `Lock`
  (set `self.Locked` true)
  (`self.ChangeColorFromLocked`))

(fn `Unlock`
  (set `self.Locked` false)
  (`self.ChangeColorFromLocked`))

(fn `UserConstructionScript`)