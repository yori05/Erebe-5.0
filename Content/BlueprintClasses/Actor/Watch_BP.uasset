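; Watch pickup actor that attaches itself to a Character_Basic on overlap.
; The first overlap calls AttachToActor, which disables both box collisions and snaps FPWatch to the character's TPMesh and TPWatch to Mesh at socket watch_r.
; It then sets IsGrabed and calls Grabed, even when the overlapping actor fails the character cast, so later overlaps are ignored.
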(event `self.ReceiveActorBeginOverlap`
  (params (OtherActor :type "Actor Object Reference"))
  (if (not (`self.IsGrabed`))
    (`self.AttachToActor` OtherActor)
    (set `self.IsGrabed` true)
    (`self.Grabed`)))

(fn `AttachToActor`
  (params (ActorTarget :type "Actor Object Reference"))
  (bind _ascharacter_basic (cast `Character_Basic` ActorTarget))
  (`PrimitiveComponent.SetCollisionEnabled` (`self.Box`) "NoCollision")
  (`PrimitiveComponent.SetCollisionEnabled` (`self.Box1`) "NoCollision")
  (`SceneComponent.K2_AttachToComponent` (`self.FP_Watch`) (`Character_Basic.TPMesh` _ascharacter_basic) "watch_r" "SnapToTarget" "SnapToTarget" "SnapToTarget" true)
  (`SceneComponent.K2_AttachToComponent` (`self.TP_Watch`) (`Character.Mesh` _ascharacter_basic) "watch_r" "SnapToTarget" "SnapToTarget" "SnapToTarget" true))

(fn `UserConstructionScript`)