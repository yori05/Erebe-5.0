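; Player controller for the Erebe character, handling HUD creation and debug and gameplay input.
; On BeginPlay it creates the HeadsUpDisplay widget and adds it to the viewport.
; The zoom axis adjusts the possessed character's camera boom arm length, clamped between fully zoomed in and a maximum distance.
; A fly-mode debug action and the G key forward to the character's Fly and DeployCable functions.
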(event `self.ReceiveBeginPlay`
  (bind _returnvalue (`|CreateWidget` "/Game/Equipement/UI/HeadsUpDisplay.HeadsUpDisplay_C"))
  (bind _output_get (set `self.HeadsUpDisplay_Widget` _returnvalue))
  (`UserWidget.AddToViewport` _output_get 0))

(event `InputAxis|ZoomAxis`
  (params (AxisValue :type "Float (single-precision)"))
  (bind _aserebe_character_bp (cast `/Game/BlueprintClasses/Character/ErebeCharacter_BP` (`self.K2_GetPawn`)))
  (bind _cameraboom (`ErebeCharacter.CameraBoom` _aserebe_character_bp))
  (bind _returnvalue (+ (* AxisValue 50.0) (`SpringArmComponent.TargetArmLength` _cameraboom)))
  (if (> _returnvalue 0.0)
    (if (< _returnvalue 300.0)
      (set `SpringArmComponent.TargetArmLength` _returnvalue _cameraboom)
      (else
        (set `SpringArmComponent.TargetArmLength` 300.0 _cameraboom)))
    (else
      (set `SpringArmComponent.TargetArmLength` 0.0 _cameraboom))))

(event `InputAction|FlyModeDebugKey`
  (params (Key :type "Key Structure"))
  (:`Pressed`
    (bind _aserebe_character_bp (cast `/Game/BlueprintClasses/Character/ErebeCharacter_BP` (`self.K2_GetPawn`)))
    (`/Game/BlueprintClasses/Character/ErebeCharacter_BP.Fly` _aserebe_character_bp)))

(event `Key|G`
  (params (Key :type "Key Structure"))
  (:`Pressed`
    (bind _aserebe_character_bp (cast `/Game/BlueprintClasses/Character/ErebeCharacter_BP` (`self.K2_GetPawn`)))
    (`/Game/BlueprintClasses/Character/ErebeCharacter_BP.DeployCable` _aserebe_character_bp)))

(fn `UserConstructionScript`)