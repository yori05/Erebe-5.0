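; Erebe character Blueprint that provides a toggle between flying and free movement states.
; Fly reads the current character state and switches between Flying and Free.
; BeginPlay, Tick and DeployCable are empty; disconnected nodes retain grapple hook logic that would spawn the hook, link it to the shooting component, attach it to the right-hand grip socket and fire it.
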(event `self.ReceiveBeginPlay`)

(event `self.ReceiveTick`
  (params (DeltaSeconds :type "Float (single-precision)")))

(fn `DeployCable`)

(fn `Fly`
  (bind _returnvalue (`self.GetCharacterState`))
  (if (`|EnumEquality` _returnvalue "CHARSTATE_Flying")
    (`self.SetCharacterState` "CHARSTATE_Free")
    (else
      (`self.SetCharacterState` "CHARSTATE_Flying"))))

(fn `UserConstructionScript`)